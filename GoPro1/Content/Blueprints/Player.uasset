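; Player car pawn for an obstacle-dodging driving game, with constant forward movement, axis-driven steering and accelerate/decelerate via FloatingPawnMovement max speed.
; Overlapping an ObstacleCar costs a life, then briefly halves forward input, locks steering, grants invulnerability and plays a timeline spin, until zero lives pauses on the game-over widget.
; Custom events handle puddle slips, pushing randomly to either side through timelines, and inverting or resetting side controls.
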(event `self.ReceiveBeginPlay`
  (bind _carmodel (`self.CarModel`))
  ;[1 1 1] Correct Height
  (`SceneComponent.K2_SetWorldLocation` _carmodel (+ (`SceneComponent.K2_GetComponentLocation` _carmodel) (0.0 0.0 -19.0)) false false))

(event `self.ReceiveTick`
  (params (DeltaSeconds :type "Float (single-precision)"))
  ;[1 1 1] Forward Movement
  (`self.AddMovementInput` (`SceneComponent.GetForwardVector` (`self.SecretSphere`)) (`self.ForwardSpeed`)))

(event `Slip`
  (bind _slipvector (`self.SlipVector`))
  ;[1 1 1] Slipping on puddle
  (set `self.CanDrive` false)
  (switch `int` (`KismetMathLibrary.RandomIntegerInRange` 0 1)
    (:`0`
      (`Timeline|Slip TimeLine` :!via `PlayFromStart`
        (:`Update`
          (`self.AddMovementInput` _slipvector 2.0))))
    (:`1`
      (`Timeline|Slip TimeLine2` :!via `PlayFromStart`
        (:`Update`
          (`self.AddMovementInput` (* _slipvector -1) 3.0)))))
  (set `self.CanDrive` true))

(event `InputAxis|Left/Right`
  (params (AxisValue :type "Float (single-precision)"))
  ;[1 1 1] Side Movement
  (if (`self.CanDrive`)
    (`self.AddMovementInput` (* (`self.SideVector`) AxisValue) (`self.SideSpeed`))))

(event `HitCar`
  ;[1 1 1] Collision Event
  (if (not (`self.IsInvulnerable`))
    (bind _result (`/Engine/EditorBlueprintResources/StandardMacros.DecrementInt` (`self.Lives`))
      (:`  `
        (if (<= _result 0)
          (`self.GameOver`)
          (else
            (set `self.IsInvulnerable` true)
            (set `self.CanDrive` false)
            (set `self.ForwardSpeed` (/ (`self.ForwardSpeed`) 2.0))
            (`self.Spin`)
            (`KismetSystemLibrary.Delay` 1.0)
            (set `self.CanDrive` true)
            (set `self.ForwardSpeed` (* (`self.ForwardSpeed`) 2.0))
            (set `self.IsInvulnerable` false)))))))

(event `InvertControls`
  ;[1 1 1] Inverting Side Controls
  (set `self.SideSpeed` -1.0))

(event `ResetControls`
  ;[1 1 1] Inverting Side Controls
  (set `self.SideSpeed` 1.0))

(event `self.Collision.OnComponentBeginOverlap`
  (params (OverlappedComponent :type "PrimitiveComponent Object Reference") (OtherActor :type "Actor Object Reference") (OtherComp :type "PrimitiveComponent Object Reference") (OtherBodyIndex :type Integer) (bFromSweep :type Boolean) (SweepResult :type "HitResult Structure (by ref)"))
  ;[1 1 1] Call Collision
  (cast `/Game/Blueprints/ObstacleCar` OtherActor)
  (`self.HitCar`))

(event `Spin`
  ;[1 1 1] Spin Animation
  (bind (_direction _spinangle) (`Timeline|SpinnyTimeline` :!via `PlayFromStart`)
    (:`Update`
      (`SceneComponent.K2_SetWorldRotation` (`self.CarModel`) (`KismetMathLibrary.MakeRotator` 0.0 0.0 (.z (`KismetMathLibrary.MakeVector` 0.0 0.0 _spinangle))) false false))))

(event `InputAction|Accelerate`
  (params (Key :type "Key Structure"))
  (bind _floatingpawnmovement (`self.FloatingPawnMovement`))
  ;[1 1 1] Speed Control
  (:`Pressed`
    (set `FloatingPawnMovement.MaxSpeed` 3000.0 _floatingpawnmovement))
  (:`Released`
    (set `FloatingPawnMovement.MaxSpeed` 2000.0 _floatingpawnmovement)))

(event `InputAction|Decelerate`
  (params (Key :type "Key Structure"))
  (bind _floatingpawnmovement (`self.FloatingPawnMovement`))
  ;[1 1 1] Speed Control
  (:`Pressed`
    (set `FloatingPawnMovement.MaxSpeed` 1000.0 _floatingpawnmovement))
  (:`Released`
    (set `FloatingPawnMovement.MaxSpeed` 2000.0 _floatingpawnmovement)))

(event `GameOver`
  ;[1 1 1] Game Over
  (bind _returnvalue (`|CreateWidget` "/Game/Blueprints/Game_Over_Widget.Game_Over_Widget_C"))
  (`UserWidget.AddToViewport` _returnvalue 0)
  (set `PlayerController.bShowMouseCursor` true (`GameplayStatics.GetPlayerController` 0))
  (`GameplayStatics.SetGamePaused` true))

(fn `UserConstructionScript`)