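; Actor that repeatedly spawns Child_Tumbleweed actors at its own root transform.
; On BeginPlay it waits a short random whole-second delay before the first spawn, so placed spawners can start out of step.
; The Spawn event then calls itself after each random delay of several seconds, forming an endless loop with no cap or cleanup.
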(event `self.ReceiveBeginPlay`
  (`KismetSystemLibrary.Delay` (`KismetMathLibrary.Conv_IntToDouble` (`KismetMathLibrary.RandomInteger` 4)))
  (`self.Spawn`))

(event `Spawn`
  (`|SpawnActorFromClass` "/Game/Blueprints/Child_Tumbleweed.Child_Tumbleweed_C" (`SceneComponent.K2_GetComponentToWorld` (`self.DefaultSceneRoot`)) "Undefined" "OverrideRootScale" null null)
  (`KismetSystemLibrary.Delay` (`KismetMathLibrary.Conv_IntToDouble` (`KismetMathLibrary.RandomIntegerInRange` 4 8)))
  (`self.Spawn`))

(fn `UserConstructionScript`)