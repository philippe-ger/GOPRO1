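; Car_Child5 is an obstacle car child Blueprint that stays put for 15 seconds after BeginPlay, then drives along world +X.
; BeginPlay holds an IsWaiting flag through the delay, and Tick moves the actor without sweep once it clears.
; Each frame's VInterpTo target is 1000 units ahead of the current location, so InterpSpeed sets a steady travel speed rather than easing to a stop.
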(event `self.ReceiveBeginPlay`
  (`parent.ReceiveBeginPlay`)
  (set `self.isWaiting` true)
  (`KismetSystemLibrary.Delay` 15.0)
  (set `self.isWaiting` false))

(event `self.ReceiveTick`
  (params (DeltaSeconds :type "Float (single-precision)"))
  (bind _returnvalue (`self.K2_GetActorLocation`))
  (`parent.ReceiveTick` DeltaSeconds)
  (if (not (`self.isWaiting`))
    (`self.K2_SetActorLocation` (`KismetMathLibrary.VInterpTo` _returnvalue (+ _returnvalue (1000.0 0.0 0.0)) DeltaSeconds (`self.InterpSpeed`)))))

(fn `UserConstructionScript`
  (`parent.UserConstructionScript`))